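; BP_TargetDummy is a shootable dummy that collapses into ragdoll physics when it takes damage.
; Any damage turns on skeletal mesh physics and makes the mesh ignore the Pawn collision channel.
; Point damage also draws a debug sphere at the hit and applies a velocity-change impulse to the struck bone along the shot direction.
; Hits to the head bone hide that bone.
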(event `self.ReceivePointDamage`
  (params (Damage :type "Float (single-precision)") (DamageType :type "DamageType Object Reference") (HitLocation :type "Vector Structure") (HitNormal :type "Vector Structure") (HitComponent :type "PrimitiveComponent Object Reference") (BoneName :type Name) (ShotFromDirection :type "Vector Structure") (InstigatedBy :type "Controller Object Reference") (DamageCauser :type "Actor Object Reference") (HitInfo :type "HitResult Structure (by ref)"))
  (bind _skeletalmesh (`self.SkeletalMesh`))
  (`KismetSystemLibrary.DrawDebugSphere` HitLocation 4.0 6 (struct :`R` 0.286458 :`G` 0.002088 :`A` 1.0) 1.0 1.0)
  (`PrimitiveComponent.SetSimulatePhysics` _skeletalmesh true)
  (`self.DisablePawnCollision`)
  (`PrimitiveComponent.AddImpulse` _skeletalmesh (* (`KismetMathLibrary.GetForwardVector` (`KismetMathLibrary.Conv_VectorToRotator` ShotFromDirection)) 750.0) BoneName true)
  (if (== BoneName "head")
    (`SkinnedMeshComponent.HideBoneByName` _skeletalmesh BoneName "PBO_None")))

(event `self.ReceiveAnyDamage`
  (params (Damage :type "Float (single-precision)") (DamageType :type "DamageType Object Reference") (InstigatedBy :type "Controller Object Reference") (DamageCauser :type "Actor Object Reference"))
  (`PrimitiveComponent.SetSimulatePhysics` (`self.SkeletalMesh`) true)
  (`self.DisablePawnCollision`))

(fn `DisablePawnCollision`
  (`PrimitiveComponent.SetCollisionResponseToChannel` (`self.SkeletalMesh`) "ECC_Pawn" "ECR_Ignore"))

(fn `UserConstructionScript`)