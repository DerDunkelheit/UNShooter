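; Player controller that opens two inventory screens for the first-person character, both driven by its InventoryComponent.
; On BeginPlay it creates and caches a grid inventory widget, which its input action toggles in the viewport, switching between Game-and-UI and game-only input with the cursor.
; A second input action creates a new WBP_Inventory on every press and switches to UI-only input, with no closing logic here.
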(event `self.ReceiveBeginPlay`
  ;[1 1 1] Create new Inventory widget, so we can use as a variable latter.
  (bind _asbp_first_person_character (cast `/Game/Blueprints/BP_FirstPersonCharacter` (`self.K2_GetPawn`)))
  (bind _returnvalue (`|CreateWidget` "/Game/Blueprints/Wigets/GridInventory/WBP_InventoryScreen_new.WBP_InventoryScreen_new_C" self (`FP_FirstPersonCharacter.InventoryComponent` _asbp_first_person_character) 70.0))
  (set `self.InventoryWIdget_new` _returnvalue))

(event `InputAction|OpenInventory`
  (params (Key :type "Key Structure"))
  (:`Pressed`
    (`self.Show Inventory UI`)))

(event `InputAction|OpenGridInventory`
  (params (Key :type "Key Structure"))
  (:`Pressed`
    (`self.ShowGridInventory`)))

(event `Show Inventory UI`
  (bind _returnvalue (`GameplayStatics.GetPlayerController` 0))
  ;[1 1 1] Input events    TODO: replace in cpp
  (bind _asbp_first_person_character (cast `/Game/Blueprints/BP_FirstPersonCharacter` (`GameplayStatics.GetPlayerCharacter` 0)))
  (bind _returnvalue_2 (`|CreateWidget` "/Game/Blueprints/Wigets/WBP_Inventory.WBP_Inventory_C" (`GameplayStatics.GetPlayerController` 0) (`FP_FirstPersonCharacter.InventoryComponent` _asbp_first_person_character)))
  (bind _output_get (set `self.Inventory Widget` _returnvalue_2))
  (`UserWidget.AddToViewport` _output_get 0)
  (set `PlayerController.bShowMouseCursor` true _returnvalue)
  (`WidgetBlueprintLibrary.SetInputMode_UIOnlyEx` _returnvalue (`self.Inventory Widget`)))

(event `ShowGridInventory`
  ;[1 1 1] Input events    TODO: replace in cpp
  (if (`Widget.IsInViewport` (`self.InventoryWIdget_new`))
    (`Widget.RemoveFromParent` (`self.InventoryWIdget_new`))
    (`WidgetBlueprintLibrary.SetInputMode_GameOnly` self)
    (set `self.bShowMouseCursor` false)
    (else
      (`UserWidget.AddToViewport` (`self.InventoryWIdget_new`) 0)
      (`WidgetBlueprintLibrary.SetInputMode_GameAndUIEx` self (`self.InventoryWIdget_new`) "DoNotLock" false)
      (set `self.bShowMouseCursor` true))))

(fn `UserConstructionScript`)