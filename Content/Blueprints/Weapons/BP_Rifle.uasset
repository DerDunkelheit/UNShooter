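; Rifle weapon Blueprint that adds firing effects and owner-death behavior.
; On fire, it attaches a muzzle emitter at the muzzle socket, plays a sound there and spawns the shell class from its AmmoComponent, ejected sideways by a velocity-change impulse.
; When the owner dies, it ends firing, detaches from the owner and enables physics simulation on its mesh.
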(event `self.ReceiveBeginPlay`)

(event `self.OnOwnerDied`
  (`self.EndFire`)
  (`self.EnablePhysics`))

(event `self.OnFire`
  (bind _meshcomponent (`self.MeshComponent`))
  (bind _muzzlesocketname (`self.MuzzleSocketName`))
  (`GameplayStatics.SpawnEmitterAttached` (`self.MuzzleEffect`) _meshcomponent _muzzlesocketname)
  (`GameplayStatics.SpawnSoundAtLocation` "/Engine/VREditor/Sounds/UI/Click_on_Button.Click_on_Button" (`SceneComponent.GetSocketLocation` _meshcomponent _muzzlesocketname) (struct) 1.0 1.0 0.0 null null)
  (`self.SpawWeaponShell`))

(fn `EnablePhysics`
  (`self.K2_DetachFromActor` "KeepWorld" "KeepWorld" "KeepWorld")
  (`PrimitiveComponent.SetSimulatePhysics` (`self.MeshComponent`) true))

(fn `SpawWeaponShell`
  (bind _shellsspawnpoint (`self.ShellsSpawnPoint`))
  (bind _returnvalue (`|SpawnActorFromClass` (`AmmoComponent.BulletShellClass` (`self.AmmoComponent`)) (`SceneComponent.K2_GetComponentToWorld` _shellsspawnpoint) "Undefined" "OverrideRootScale" null null))
  (`PrimitiveComponent.AddImpulse` (`self.GetComponentByClass` _returnvalue "/Script/Engine.StaticMeshComponent") (* (`SceneComponent.GetRightVector` _shellsspawnpoint) 150.0) "None" true))

(fn `UserConstructionScript`)