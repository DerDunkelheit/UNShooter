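; Enemy AI character Blueprint that wanders the level and ragdolls on death.
; A looping timer sends it to random reachable navmesh points, while an unconnected behavior tree setup never runs.
; Point damage records the hit bone and shot impulse, which Die applies after disabling capsule collision and enabling mesh physics.
; Further hits push the simulated ragdoll, and initial weapon setup runs on BeginPlay.
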(event `self.ReceiveBeginPlay`
  (`self.SetupInitialWeapon`)
  (`KismetSystemLibrary.K2_SetTimerDelegate` (delegate `Random Wander`) 1.5 true))

(event `Random Wander`
  (`AIBlueprintHelperLibrary.SimpleMoveToLocation` (`self.GetController`) (`NavigationSystemV1.K2_GetRandomReachablePointInRadius` (`self.K2_GetActorLocation`) 5000.0 null null)))

(event `self.DieEvent`
  (`self.Die`))

(event `self.ReceivePointDamage`
  (params (Damage :type "Float (single-precision)") (DamageType :type "DamageType Object Reference") (HitLocation :type "Vector Structure") (HitNormal :type "Vector Structure") (HitComponent :type "PrimitiveComponent Object Reference") (BoneName :type Name) (ShotFromDirection :type "Vector Structure") (InstigatedBy :type "Controller Object Reference") (DamageCauser :type "Actor Object Reference") (HitInfo :type "HitResult Structure (by ref)"))
  (bind _mesh (`self.Mesh`))
  (bind _output_get (set `self.LastHitBone` BoneName))
  (`KismetSystemLibrary.PrintString` (`KismetStringLibrary.Conv_NameToString` BoneName))
  (bind _output_get_2 (set `self.LastShotVector` (* (`KismetMathLibrary.GetForwardVector` (`KismetMathLibrary.Conv_VectorToRotator` ShotFromDirection)) 750.0)))
  (if (`SceneComponent.IsSimulatingPhysics` _mesh "None")
    (`PrimitiveComponent.AddImpulse` _mesh _output_get_2 _output_get true)))

(fn `Die`
  (`PrimitiveComponent.SetCollisionEnabled` (`self.CapsuleComponent`) "NoCollision")
  (`PrimitiveComponent.SetSimulatePhysics` (`self.Mesh`) true)
  (`PrimitiveComponent.AddImpulse` (`self.Mesh`) (`self.LastShotVector`) (`self.LastHitBone`) true))

(fn `UserConstructionScript`)