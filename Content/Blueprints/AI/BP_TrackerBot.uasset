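; BP_TrackerBot is an explosive AI bot that self-destructs when it dies or shortly after a ThirdPersonCharacter enters its detection area, following a warning sound.
; The explosion spawns effects, applies full radial damage using ExplosionRadius as base damage, fires a radial force impulse and destroys the actor.
; Taking damage timestamps a new dynamic material instance to trigger a glow.
; Tick draws a debug sphere at ExplosionRadius, which excludes the damage radius offset.
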(event `self.ReceiveBeginPlay`)

(event `self.ReceiveTick`
  (params (DeltaSeconds :type "Float (single-precision)"))
  (`KismetSystemLibrary.DrawDebugSphere` (`self.K2_GetActorLocation`) (`self.ExplosionRadius`) 12 (struct :`R` 1.0 :`G` 1.0 :`B` 1.0 :`A` 1.0) 0.0 1.0))

(event `self.DieEvent`
  ;[1 1 1] Events implementation
  (`self.SelfDestory`))

(event `self.ReceiveAnyDamage`
  (params (Damage :type "Float (single-precision)") (DamageType :type "DamageType Object Reference") (InstigatedBy :type "Controller Object Reference") (DamageCauser :type "Actor Object Reference"))
  ;[1 1 1] Events implementation
  (`self.EnableGlowInMaterial`))

(event `self.PlayerDetectArea.OnComponentBeginOverlap`
  (params (OverlappedComponent :type "PrimitiveComponent Object Reference") (OtherActor :type "Actor Object Reference") (OtherComp :type "PrimitiveComponent Object Reference") (OtherBodyIndex :type Integer) (bFromSweep :type Boolean) (SweepResult :type "HitResult Structure (by ref)"))
  (cast `/Game/Blueprints/ThirdPersonCharacter` OtherActor)
  (`GameplayStatics.PlaySoundAtLocation` "/Game/Assets/Sounds/DroneTracker_explodewarning.DroneTracker_explodewarning" (`self.K2_GetActorLocation`) (struct) 1.0 1.0 0.0 null null null)
  (`KismetSystemLibrary.Delay` 0.4)
  (`self.SelfDestory`))

(fn `EnableGlowInMaterial`
  (bind _meshcomponent (`self.MeshComponent`))
  (bind _returnvalue (`PrimitiveComponent.CreateDynamicMaterialInstance` _meshcomponent 0 (`PrimitiveComponent.GetMaterial` _meshcomponent 0) "None"))
  (bind _output_get (set `self.MatInst` _returnvalue))
  (`MaterialInstanceDynamic.SetScalarParameterValue` _output_get "LastTimeDamageTaken" (`GameplayStatics.GetTimeSeconds`)))

(fn `SelfDestory`
  (bind _returnvalue (`self.K2_GetActorLocation`))
  (`GameplayStatics.SpawnEmitterAtLocation` "/Game/Assets/StarterContent/Particles/P_Explosion.P_Explosion" _returnvalue)
  (`GameplayStatics.SpawnSoundAtLocation` "/Game/Assets/StarterContent/Audio/Explosion01.Explosion01" _returnvalue (struct) 1.0 1.0 0.0 null null)
  (`GameplayStatics.ApplyRadialDamage` (`self.ExplosionRadius`) _returnvalue (+ (`self.ExplosionRadius`) (`self.ExplosionRadiusOffset`)) null (`|MakeArray` self :!type "Actor Object Reference") null null true)
  (`RadialForceComponent.FireImpulse` (`self.RadialForceComponent`))
  (`self.K2_DestroyActor`))

(fn `UserConstructionScript`)