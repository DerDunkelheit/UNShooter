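; A test actor for the Minecraft-style crafting system that exercises the crafting manager and a dialog component.
; On BeginPlay it fetches the crafting manager from the custom game instance and calls its test function.
; Debug keys G and K show the next dialog and send dialogues through the DialogComponent.
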(event `self.ReceiveBeginPlay`
  (bind _asbp_custome_game_instance (cast `/Game/Blueprints/BP_CustomeGameInstance` (`GameplayStatics.GetGameInstance`)))
  (bind _asbp_crafting_manger (cast `/Game/Blueprints/MinecraftCraftingSystem/Managers/BP_CraftingManger` (`CustomGameInstance.CraftingManager` _asbp_custome_game_instance)))
  (`/Game/Blueprints/MinecraftCraftingSystem/Managers/BP_CraftingManger.BpTestFunction` _asbp_crafting_manger))

(event `Key|G`
  (params (Key :type "Key Structure"))
  (:`Pressed`
    (`DialogComponent.ShowNextDialog` (`self.DialogComponent`))))

(event `Key|K`
  (params (Key :type "Key Structure"))
  (:`Pressed`
    (`DialogComponent.SendDialogues` (`self.DialogComponent`))))

(fn `UserConstructionScript`)