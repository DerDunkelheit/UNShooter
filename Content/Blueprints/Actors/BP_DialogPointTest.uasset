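; BP_DialogPointTest is a test actor that offers dialogue when the TPPShooterCharacter enters its interaction range.
; It gets the DialoguesManager from BP_CustomeGameInstance and binds to its start and end events to track dialogue state with debug prints.
; Overlap begin sends the Dialog component's lines to the manager, and overlap end clears them.
; Interact advances the dialogue, resending the lines first if none has started.
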(event `self.ReceiveBeginPlay`
  (bind _dialoguesmanager (`self.DialoguesManager`))
  (`self.SetupDialogManager`)
  (add `DialoguesManager.DialogStartedEvent` _dialoguesmanager (delegate `OnDialogStarted`))
  (add `DialoguesManager.DialogEndedEvent` _dialoguesmanager (delegate `OnDialogEnded`)))

(event `OnDialogEnded`
  (`KismetSystemLibrary.PrintString` "OnDialogEnded" true true (struct :`R` 1.0 :`G` 0.913726 :`B` 0.094118 :`A` 1.0))
  (set `self.WasDialogStarted` false))

(event `OnDialogStarted`
  (`KismetSystemLibrary.PrintString` "OnDIalogStarted" true true (struct :`R` 1.0 :`G` 0.90864 :`B` 0.09783 :`A` 1.0))
  (set `self.WasDialogStarted` true))

(event `self.Interact`
  (`self.Handle Dialogs`))

(event `self.InteractionRange.OnComponentBeginOverlap`
  (params (OverlappedComponent :type "PrimitiveComponent Object Reference") (OtherActor :type "Actor Object Reference") (OtherComp :type "PrimitiveComponent Object Reference") (OtherBodyIndex :type Integer) (bFromSweep :type Boolean) (SweepResult :type "HitResult Structure (by ref)"))
  (cast `TPPShooterCharacter` OtherActor)
  (`DialogComponent.SendDialogues` (`self.Dialog`)))

(event `self.InteractionRange.OnComponentEndOverlap`
  (params (OverlappedComponent :type "PrimitiveComponent Object Reference") (OtherActor :type "Actor Object Reference") (OtherComp :type "PrimitiveComponent Object Reference") (OtherBodyIndex :type Integer))
  (cast `TPPShooterCharacter` OtherActor)
  (`DialoguesManager.ClearDialogues` (`self.DialoguesManager`)))

(fn `BindEvents`)

(fn `Handle Dialogs`
  (bind _dialoguesmanager (`self.DialoguesManager`))
  (if (`self.WasDialogStarted`)
    (`DialoguesManager.ShowNextDialog` _dialoguesmanager)
    (else
      (`DialogComponent.SendDialogues` (`self.Dialog`))
      (`DialoguesManager.ShowNextDialog` _dialoguesmanager))))

(fn `SetupDialogManager`
  (bind _asbp_custome_game_instance (cast `/Game/Blueprints/BP_CustomeGameInstance` (`GameplayStatics.GetGameInstance`)))
  (set `self.DialoguesManager` (`CustomGameInstance.DialoguesManager` _asbp_custome_game_instance)))

(fn `UserConstructionScript`)