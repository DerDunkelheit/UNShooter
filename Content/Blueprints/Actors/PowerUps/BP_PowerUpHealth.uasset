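; Health power-up actor that restores the player's health when interacted with.
; On Interact it calls HealPlayer, plays a pickup sound and destroys itself.
; HealPlayer casts player character 0 to FirstPersonCharacter, restores RestoreAmount through its HealthComponent and prints the resulting health to screen.
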(event `self.Interact`
  (`self.HealPlayer`)
  (`self.PlayPickUpSound`)
  (`self.K2_DestroyActor`))

(fn `HealPlayer`
  (bind _asfirst_person_character (cast `/Game/Blueprints/FirstPersonCharacter` (`GameplayStatics.GetPlayerCharacter` 0)))
  (bind _healthcomponent (`FP_FirstPersonCharacter.HealthComponent` _asfirst_person_character))
  (`HealthComponent.RestoreHealth` _healthcomponent (`self.RestoreAmount`))
  (bind _returnvalue (`HealthComponent.GetCurrentHealth` _healthcomponent))
  (`KismetSystemLibrary.PrintString` (`KismetTextLibrary.Conv_TextToString` (`|FormatText` "Current health: {currentHealth}" _returnvalue))))

(fn `UserConstructionScript`)