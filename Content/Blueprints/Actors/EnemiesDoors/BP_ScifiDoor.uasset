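; BP_ScifiDoor is a sci-fi door actor that opens when its room is cleared.
; On BeginPlay it caches the AnimBP_scifiDoor instance from its skeletal door mesh.
; OnRoomCleared and CloseDoor set that AnimBP's OpenDoor flag, leaving the door's motion to the animation Blueprint.
; The G and C keys also open and close it directly.
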(event `self.ReceiveBeginPlay`
  (bind _asanim_bp_scifi_door (cast `/Game/Animation/AnimationsBP/AnimBP_scifiDoor` (`SkeletalMeshComponent.GetAnimInstance` (`self.SkeletalDoorMesh`))))
  (set `self.BP_ScifiDoor` _asanim_bp_scifi_door))

(event `self.CloseDoor`
  ;[1 1 1] Events implementations
  (set `/Game/Animation/AnimationsBP/AnimBP_scifiDoor.bOpenDoor` false (`self.BP_ScifiDoor`)))

(event `Key|G`
  (params (Key :type "Key Structure"))
  ;[1 1 1] Inputs
  (:`Pressed`
    (set `/Game/Animation/AnimationsBP/AnimBP_scifiDoor.bOpenDoor` true (`self.BP_ScifiDoor`))))

(event `Key|C`
  (params (Key :type "Key Structure"))
  ;[1 1 1] Inputs
  (:`Pressed`
    (set `/Game/Animation/AnimationsBP/AnimBP_scifiDoor.bOpenDoor` false (`self.BP_ScifiDoor`))))

(event `self.OnRoomCleared`
  ;[1 1 1] Events implementations
  (set `/Game/Animation/AnimationsBP/AnimBP_scifiDoor.bOpenDoor` true (`self.BP_ScifiDoor`)))

(fn `UserConstructionScript`)