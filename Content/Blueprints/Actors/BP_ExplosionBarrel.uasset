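; BP_ExplosionBarrel is an exploding barrel actor that deals area damage and pushes objects with a radial force.
; SelfDestroy spawns particle and sound effects, destroys the mesh, applies full radial damage, fires the RadialForce impulse, then destroys the actor; nothing here calls it.
; ExplosionRadius drives both damage and force radius, with effects and damage centred on DestroyEmmiterPosition.
; Tick draws a debug sphere showing that radius.
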(event `self.ReceiveBeginPlay`
  (set `RadialForceComponent.Radius` (`self.ExplosionRadius`) (`self.RadialForce`)))

(event `self.ReceiveTick`
  (params (DeltaSeconds :type "Float (single-precision)"))
  (`KismetSystemLibrary.DrawDebugSphere` (`SceneComponent.K2_GetComponentLocation` (`self.DestroyEmmiterPosition`)) (`self.ExplosionRadius`) 12 (struct :`R` 0.4375 :`B` 0.006098 :`A` 1.0)))

(event `self.SelfDestroy`
  (`self.Explosion`)
  (`self.CastRadialDamage`)
  (`RadialForceComponent.FireImpulse` (`self.RadialForce`))
  (`self.K2_DestroyActor`))

(fn `CastRadialDamage`
  (`GameplayStatics.ApplyRadialDamage` :`BaseDamage` (`self.ExplosionDamage`) :`Origin` (`SceneComponent.K2_GetComponentLocation` (`self.DestroyEmmiterPosition`)) :`DamageRadius` (`self.ExplosionRadius`) :`DamageCauser` null :`InstigatedByController` null :`bDoFullDamage` true))

(fn `Explosion`
  (bind _returnvalue (`SceneComponent.K2_GetComponentLocation` (`self.DestroyEmmiterPosition`)))
  (`GameplayStatics.SpawnEmitterAtLocation` (`self.DestroyParticle`) _returnvalue)
  (`GameplayStatics.SpawnSoundAtLocation` (`self.DestroySoundWave`) _returnvalue (struct) 1.0 1.0 0.0 null null)
  (`ActorComponent.K2_DestroyComponent` (`self.MeshComponent`)))

(fn `UserConstructionScript`)