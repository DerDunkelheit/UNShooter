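; Remote camera controller that, on Interact, hands the player's possession over to a controlled camera pawn.
; BeginPlay caches the pawn at index 0 as the last controlled pawn.
; Interact loops over all controlled pawns, storing the player's current pawn as each one's previous pawn and possessing that cached pawn on every pass.
; An empty pawn list prints a red error instead.
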(event `self.ReceiveBeginPlay`
  (bind _returnvalue (`self.GetControlledPawnByIndex` 0))
  (`self.SetLastControlledPawn` _returnvalue))

(event `self.Interact`
  (if (> (`KismetArrayLibrary.Array_Length` (`self.ControlledPawns`)) 0)
    (`KismetSystemLibrary.PrintString` (`KismetTextLibrary.Conv_TextToString` (`|FormatText` "Controlled cameras {count}" (`KismetArrayLibrary.Array_Length` (`self.ControlledPawns`)))))
    (for _array_element (`self.ControlledPawns`)
      (`RemotelyControlledPawn.SetPreviousPawn` _array_element (`Controller.K2_GetPawn` (`GameplayStatics.GetPlayerController` 0)))
      (`Controller.Possess` (`GameplayStatics.GetPlayerController` 0) (`self.LastControlledPawn`)))
    (else
      (`KismetSystemLibrary.PrintString` "Controlled pawn is nullpnt, you have to assign it" true true (struct :`R` 0.854167 :`A` 1.0)))))

(fn `UserConstructionScript`)