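; BP_RemoteTurret is a possessable remote-control turret with its own HUD and camera.
; On possession it clamps camera yaw to a forward arc, shows the HUD and sets control rotation from LastPawnRotator.
; On unpossession, if the HUD is valid, it removes it and copies the camera's relative transform to the scene capture.
; Each tick, the camera interpolates toward the skeletal mesh's CameraPointSocket.
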(event `self.OnTurretPossessed`
  (params (NewPawn :type "Pawn Object Reference"))
  (bind _returnvalue (`GameplayStatics.GetPlayerCameraManager` 0))
  (if (== NewPawn self)
    (set `PlayerCameraManager.ViewYawMin` -45.0 _returnvalue)
    (set `PlayerCameraManager.ViewYawMax` 45.0 _returnvalue)
    (bind _returnvalue_2 (`|CreateWidget` "/Game/Blueprints/Actors/Features/RemoteControl/WBP_RemoteTurretHUD.WBP_RemoteTurretHUD_C"))
    (bind _output_get (set `self.RemoteTurretHUD` _returnvalue_2))
    (`UserWidget.AddToViewport` _output_get 0)
    (`Controller.SetControlRotation` (`GameplayStatics.GetPlayerController` 0) (`self.LastPawnRotator`))))

(event `self.OnTurretUnPossessed`
  (bind _remoteturrethud (`self.RemoteTurretHUD`))
  ;[1 1 1] Remove Turret hud and update scene capture Transform
  (`/Engine/EditorBlueprintResources/StandardMacros.IsValid` _remoteturrethud
    (:`Is Valid`
      (`Widget.RemoveFromParent` _remoteturrethud)
      (`SceneComponent.K2_SetRelativeTransform` (`self.SceneCaptureComponent`) (`SceneComponent.GetRelativeTransform` (`self.CameraComponent`)) false false))))

(event `self.ReceiveTick`
  (params (DeltaSeconds :type "Float (single-precision)"))
  ;[1 1 1] Update Camera Location
  (`SceneComponent.K2_SetWorldLocation` (`self.CameraComponent`) (`KismetMathLibrary.VInterpTo` (`SceneComponent.K2_GetComponentLocation` (`self.CameraComponent`)) (`SceneComponent.GetSocketLocation` (`self.SkeletalMeshComponent`) "CameraPointSocket") (`GameplayStatics.GetWorldDeltaSeconds`) 30.0) false false))

(fn `UserConstructionScript`)