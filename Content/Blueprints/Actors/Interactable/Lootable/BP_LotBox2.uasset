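; BP_LotBox2 is an interactable sci-fi loot container that opens a loot inventory screen.
; On BeginPlay it caches its skeletal mesh's AnimBP_scifi_container3 instance and the first-person player character.
; Interact sets the open flag on the anim blueprint, creates WBP_InventoryLootActor with its InventoryComponent and switches to UI-only input with the cursor shown.
; The widget's close event is bound to clear the flag, triggering the close animation.
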(event `self.ReceiveBeginPlay`
  (`self.SetAnimaBPVariable`)
  (`self.SetPlayerVariable`))

(event `self.Interact`
  (bind _returnvalue (`GameplayStatics.GetPlayerController` 0))
  (set `/Game/Animation/AnimationsBP/AnimBP_scifi_container3.bOpenContainer` true (`self.AnimBP_Container3`))
  (bind _returnvalue_2 (`|CreateWidget` "/Game/Blueprints/Wigets/LootWidgets/WBP_InventoryLootActor.WBP_InventoryLootActor_C" (`GameplayStatics.GetPlayerController` 0) null (`self.InventoryComponent`)))
  (`UserWidget.AddToViewport` _returnvalue_2 0)
  (add `InventoryWidgetBase.CloseWidgetEvent` _returnvalue_2 (delegate `TriggerCloseAnimation`))
  (set `PlayerController.bShowMouseCursor` true _returnvalue)
  (`WidgetBlueprintLibrary.SetInputMode_UIOnlyEx` _returnvalue _returnvalue_2))

(event `TriggerCloseAnimation`
  (set `/Game/Animation/AnimationsBP/AnimBP_scifi_container3.bOpenContainer` false (`self.AnimBP_Container3`)))

(fn `SetAnimaBPVariable`
  (bind _asanim_bp_scifi_container_3 (cast `/Game/Animation/AnimationsBP/AnimBP_scifi_container3` (`SkeletalMeshComponent.GetAnimInstance` (`self.SkeletalMeshComponent`))))
  (set `self.AnimBP_Container3` _asanim_bp_scifi_container_3))

(fn `SetPlayerVariable`
  (bind _asfirst_person_character (cast `/Game/Blueprints/FirstPersonCharacter` (`GameplayStatics.GetPlayerCharacter` 0)))
  (set `self.MainCharacter` _asfirst_person_character))

(fn `UserConstructionScript`)